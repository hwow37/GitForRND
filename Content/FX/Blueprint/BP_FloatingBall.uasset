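; BP_FloatingBall is an FX actor that configures the Niagara component NSFloatingBallBlockingArea, apparently a floating-ball effect for blocking areas.
; It forwards its variables for random movement, upward gravity and size ranges to the effect's float parameters.
; BeginPlay sets the full min/max ranges.
; The construction script does likewise, except it writes MinGravityUp to a single GravityUp parameter and omits MaxGravityUp.
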(event EventBeginPlay
  (bind _ns_floatingball_blockingarea (Variables|Default|GetNS_FloatingBall_BlockingArea))
  (Niagara|SetNiagaraVariable(Float) _ns_floatingball_blockingarea "MinMoveRandom" (Variables|InitVFX|GetMinMoveRandom))
  (Niagara|SetNiagaraVariable(Float) _ns_floatingball_blockingarea "MaxMoveRandom" (Variables|InitVFX|GetMaxMoveRandom))
  (Niagara|SetNiagaraVariable(Float) _ns_floatingball_blockingarea "MinGravityUp" (Variables|InitVFX|GetMinGravityUp))
  (Niagara|SetNiagaraVariable(Float) _ns_floatingball_blockingarea "MaxGravityUp" (Variables|InitVFX|GetMaxGravityUp))
  (Niagara|SetNiagaraVariable(Float) _ns_floatingball_blockingarea "MinSize" (Variables|InitVFX|GetMinSize))
  (Niagara|SetNiagaraVariable(Float) _ns_floatingball_blockingarea "MaxSize" (Variables|InitVFX|GetMaxSize)))

(event Collision|EventActorBeginOverlap
  (params (OtherActor :type Actor%20Object%20Reference)))

(event EventTick
  (params (DeltaSeconds :type Float%20%28single-precision%29)))

(fn ConstructionScript
  (bind _ns_floatingball_blockingarea (Variables|Default|GetNS_FloatingBall_BlockingArea))
  (Niagara|SetNiagaraVariable(Float) _ns_floatingball_blockingarea "MinMoveRandom" (Variables|InitVFX|GetMinMoveRandom))
  (Niagara|SetNiagaraVariable(Float) _ns_floatingball_blockingarea "MaxMoveRandom" (Variables|InitVFX|GetMaxMoveRandom))
  (Niagara|SetNiagaraVariable(Float) _ns_floatingball_blockingarea "GravityUp" (Variables|InitVFX|GetMinGravityUp))
  (Niagara|SetNiagaraVariable(Float) _ns_floatingball_blockingarea "MinSize" (Variables|InitVFX|GetMinSize))
  (Niagara|SetNiagaraVariable(Float) _ns_floatingball_blockingarea "MaxSize" (Variables|InitVFX|GetMaxSize)))