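; BP_Waterfall_Bottom is a waterfall base effect pairing a Niagara system with a water decal.
; The construction script pushes per-axis scale and spawn rate variables into the Niagara system and sets the decal's world scale.
; BeginPlay resends the Niagara values, but names the spawn rate "SetSpawnrRate" instead of the construction script's "SetSpawnRate".
; A decal material call exists but never runs.
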(event EventBeginPlay
  (bind _ns_waterfall_bottom_type02 (Variables|Default|GetNS_Waterfall_Bottom_Type02))
  (Niagara|SetNiagaraVariable(Float) _ns_waterfall_bottom_type02 "ScaleX" (Variables|Default|GetScaleX))
  (Niagara|SetNiagaraVariable(Float) _ns_waterfall_bottom_type02 "ScaleY" (Variables|Default|GetScaleY))
  (Niagara|SetNiagaraVariable(Float) _ns_waterfall_bottom_type02 "ScaleZ" (Variables|Default|GetScaleZ))
  (Niagara|SetNiagaraVariable(Float) _ns_waterfall_bottom_type02 "SetSpawnrRate" (Variables|Default|GetSpawnRate)))

(event Collision|EventActorBeginOverlap
  (params (OtherActor :type Actor%20Object%20Reference)))

(event EventTick
  (params (DeltaSeconds :type Float%20%28single-precision%29)))

(fn ConstructionScript
  (bind _ns_waterfall_bottom_type02 (Variables|Default|GetNS_Waterfall_Bottom_Type02))
  (Utilities|FlowControl|Sequence
    (:then_0
      (Niagara|SetNiagaraVariable(Float) _ns_waterfall_bottom_type02 "ScaleX" (Variables|Default|GetScaleX))
      (Niagara|SetNiagaraVariable(Float) _ns_waterfall_bottom_type02 "ScaleY" (Variables|Default|GetScaleY))
      (Niagara|SetNiagaraVariable(Float) _ns_waterfall_bottom_type02 "ScaleZ" (Variables|Default|GetScaleZ))
      (Niagara|SetNiagaraVariable(Float) _ns_waterfall_bottom_type02 "SetSpawnRate" (Variables|Default|GetSpawnRate)))
    (:then_1
      (Transformation|SetWorldScale3D (Variables|Default|GetDecal_Water) (Variables|Default|GetDecalScale)))))