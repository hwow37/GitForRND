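; Waterfall effect actor that builds a chain of spline meshes along its spline in the Construction Script, with no runtime logic.
; Each segment follows the spline points and tangents and widens cumulatively by ScaleUp, with the final segment spawned from a separate component node.
; Materials receive a shared random TimeOffset to vary timing and the segment index as MeshUV_Y, and decals are disabled.
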(event EventBeginPlay)

(event Collision|EventActorBeginOverlap
  (params (OtherActor :type Actor%20Object%20Reference)))

(event EventTick
  (params (DeltaSeconds :type Float%20%28single-precision%29)))

(fn ConstructionScript
  (bind _spline (Variables|Default|GetSpline))
  (bind _spline_2 (Variables|Default|GetSpline))
  (bind _spline_3 (Variables|Default|GetSpline))
  (bind _scaleup (Variables|Default|GetScaleUp))
  (bind _returnvalue (Spline|GetNumberOfSplinePoints _spline))
  (bind _returnvalue_2 (- _returnvalue 2))
  (Variables|Default|SetTimeOffset (Math|Random|RandomFloatinRange 0.0 1e+01))
  (for _index (range 0 _returnvalue_2)
    (if (not (== _returnvalue_2 _index))
      (bind _returnvalue_3 (AddComponent|AddSplineMeshComponent false))
      (SplineMesh|SetForwardAxis _returnvalue_3 "Y" true)
      (SplineMesh|SetStartScale _returnvalue_3 (+ "(X=1.000000,Y=1.000000)" (* _scaleup (Math|Conversions|ToFloat(Integer) _index))) true :!class /Script/Engine.SplineMeshComponent)
      (SplineMesh|SetEndScale _returnvalue_3 (+ "(X=1.000000,Y=1.000000)" (* _scaleup (+ (Math|Conversions|ToFloat(Integer) _index) 1.0))) true :!class /Script/Engine.SplineMeshComponent)
      (SplineMesh|SetStartandEnd _returnvalue_3 (Spline|GetLocationatSplinePoint _spline_3 _index "Local") (Spline|GetTangentatSplinePoint _spline_3 _index "Local") (Spline|GetLocationatSplinePoint _spline_2 (+ _index 1) "Local") (Spline|GetTangentatSplinePoint _spline_2 (+ _index 1) "Local") true :!class /Script/Engine.SplineMeshComponent)
      (Rendering|Material|SetScalarParameterValueonMaterials _returnvalue_3 "TimeOffset" (Variables|Default|GetTimeOffset))
      (Rendering|Material|SetScalarParameterValueonMaterials _returnvalue_3 "MeshUV_Y" (Math|Conversions|ToFloat(Integer) _index))
      (Rendering|SetReceivesDecals _returnvalue_3 false)
      (else
        (bind _returnvalue_4 (AddComponent|AddSplineMeshComponent false))
        (SplineMesh|SetForwardAxis _returnvalue_4 "Y" true)
        (SplineMesh|SetStartScale _returnvalue_4 (+ "(X=1.000000,Y=1.000000)" (* _scaleup (Math|Conversions|ToFloat(Integer) _index))) true :!class /Script/Engine.SplineMeshComponent)
        (SplineMesh|SetEndScale _returnvalue_4 (+ "(X=1.000000,Y=1.000000)" (* _scaleup (+ (Math|Conversions|ToFloat(Integer) _index) 1.0))) true :!class /Script/Engine.SplineMeshComponent)
        (SplineMesh|SetStartandEnd _returnvalue_4 (Spline|GetLocationatSplinePoint _spline_3 _index "Local") (Spline|GetTangentatSplinePoint _spline_3 _index "Local") (Spline|GetLocationatSplinePoint _spline_2 (+ _index 1) "Local") (Spline|GetTangentatSplinePoint _spline_2 (+ _index 1) "Local") true :!class /Script/Engine.SplineMeshComponent)
        (Rendering|Material|SetScalarParameterValueonMaterials _returnvalue_4 "TimeOffset" (Variables|Default|GetTimeOffset))
        (Rendering|Material|SetScalarParameterValueonMaterials _returnvalue_4 "MeshUV_Y" (Math|Conversions|ToFloat(Integer) _index))
        (Rendering|SetReceivesDecals _returnvalue_4 false)))))